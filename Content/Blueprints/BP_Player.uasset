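; BP_Player is the player character, with Enhanced Input movement, look, firing and switching between a pistol and a rifle.
; BeginPlay adds the mapping context and spawns the pistol.
; SpawnWeapon destroys the current weapon and attaches a new one to the mesh's right-hand pistol socket, which both weapons share.
; Fire calls the current weapon and plays a montage chosen by the HoldingRifle flag, which switching toggles.
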(event Input|EnhancedActionEvents|EnhancedInputActionIA_Move
  (params (ActionValue :type Vector%202D%20Structure) (ElapsedSeconds :type Float%20%28double-precision%29) (TriggeredSeconds :type Float%20%28double-precision%29) (InputAction :type Input%20Action%20Object%20Reference :default "/Game/Input/IA_Move.IA_Move"))
  (Pawn|Input|AddMovementInput (Transformation|GetActorForwardVector) (.y ActionValue) false)
  (Pawn|Input|AddMovementInput (Transformation|GetActorRightVector) (.x ActionValue) false))

(event Input|EnhancedActionEvents|EnhancedInputActionIA_Look
  (params (ActionValue :type Vector%202D%20Structure) (ElapsedSeconds :type Float%20%28double-precision%29) (TriggeredSeconds :type Float%20%28double-precision%29) (InputAction :type Input%20Action%20Object%20Reference :default "/Game/Input/IA_Look.IA_Look"))
  (Pawn|Input|AddControllerYawInput (.x ActionValue))
  (Pawn|Input|AddControllerPitchInput (* (.y ActionValue) -1.0)))

(event Input|EnhancedActionEvents|EnhancedInputActionIA_Fire
  (params (ActionValue :type Boolean) (ElapsedSeconds :type Float%20%28double-precision%29) (TriggeredSeconds :type Float%20%28double-precision%29) (InputAction :type Input%20Action%20Object%20Reference :default "/Game/Input/IA_Fire.IA_Fire"))
  (:Started
    (bind _current_weapon (Variables|Default|GetCurrent%20Weapon)
      (:then
        (Default|Fire _current_weapon)
        (if (Variables|Default|GetHoldingRifle)
          (Animation|PlayAnimMontage "/Game/Rifle_01/Animation/In-Place/W2_Stand_Fire_Single_IPC_Montage.W2_Stand_Fire_Single_IPC_Montage" 1.0 "None")
          (else
            (Animation|PlayAnimMontage "/Game/Pistol_Basic/Animation/Holster_and_Fire/W1_Stand_Fire_Single_Montage.W1_Stand_Fire_Single_Montage" 1.0 "None"))))
      (:else))))

(event Input|EnhancedActionEvents|EnhancedInputActionIA_SwitchWeapon
  (params (ActionValue :type Boolean) (ElapsedSeconds :type Float%20%28double-precision%29) (TriggeredSeconds :type Float%20%28double-precision%29) (InputAction :type Input%20Action%20Object%20Reference :default "/Game/Input/IA_SwitchWeapon.IA_SwitchWeapon"))
  (:Started
    (if (Variables|Default|GetHoldingRifle)
      (CallFunction|SpawnWeapon (Variables|Default|GetPistol))
      (Variables|Default|SetHoldingRifle false)
      (else
        (CallFunction|SpawnWeapon (Variables|Default|GetRifle))
        (Variables|Default|SetHoldingRifle true)))))

(event EventBeginPlay
  (Input|AddMappingContext (PlayerController|LocalPlayerSubsystems|GetEnhancedInputLocalPlayerSubsystem (Game|GetPlayerController 0)) "/Game/Input/InputMappingContext.InputMappingContext" 0 "(bIgnoreAllPressedKeysUntilRelease=True,bForceImmediately=False,bNotifyUserSettings=False)")
  (CallFunction|SpawnWeapon (Variables|Default|GetPistol)))

(fn ConstructionScript)

(fn SpawnWeapon
  (params (Weapon%20To%20Spawn :type BP%20Weapon%20Class%20Reference))
  (bind _current_weapon (Variables|Default|GetCurrent%20Weapon)
    (:then
      (Actor|DestroyActor _current_weapon))
    (:else
      _))
  (bind _returnvalue (Game|SpawnActorfromClass Weapon%20To%20Spawn (Transformation|GetSocketTransform (Variables|Character|GetMesh) "hand_r_PistolSocket" "RTS_World") "Undefined" "MultiplyWithRoot" 0 0))
  (Transformation|AttachComponentToComponent _returnvalue (Variables|Character|GetMesh) "hand_r_PistolSocket" "SnapToTarget" "SnapToTarget" "KeepWorld" true)
  (Variables|Default|SetCurrent%20Weapon _returnvalue))